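; RTS NPC Blueprint that gives each character a random identity and its own HUD widget.
; The construction script picks one of two sexes, tints a dynamic body material and stores a random name drawn from that sex's name enum.
; BeginPlay binds to the camera controller's HUD request, and DisplayHud shows the widget only when this NPC is the requested actor.
; SetIsBusy writes a busy flag to the AI blackboard.
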(event `self.ReceiveBeginPlay`
  (set `self.AiControllerRef` (cast `/Game/RTS/AI/NPC_AIController` (`AIBlueprintHelperLibrary.GetAIController` null) :!pure true))
  (bind _ascamera_pawn_controller (cast `/Game/RTS/Blueprints/CameraPawnController` (`GameplayStatics.GetPlayerController` 0)))
  (bind _output_get (set `self.CameraControllerRef` _ascamera_pawn_controller))
  (add `/Game/RTS/Blueprints/CameraPawnController.HudRequest` _output_get (`|CreateDelegate` :!event `DisplayHud`))
  (bind _returnvalue (`|CreateWidget` "/Game/RTS/HUDs/NPC_Hud.NPC_Hud_C"))
  (set `self.NPC_HUD` _returnvalue))

(event `DisplayHud`
  (params (Actor :type "Actor Object Reference"))
  (if (== Actor self)
    (`UserWidget.AddToViewport` (`self.NPC_HUD`) 0)))

(fn `GetRandomName`
  (params (Sex :type Byte :default 0))
  (returns (Name :type String))
  (if (`|EnumEquality` Sex)
    (return (`|GetEnumeratorNameAsString` (enumliteral `/Game/RTS/Enums/MaleNameEnum` (cast `/Game/RTS/Enums/MaleNameEnum` (`KismetMathLibrary.Conv_IntToByte` (`KismetMathLibrary.RandomIntegerInRange` 0 (- (enumcount `/Game/RTS/Enums/MaleNameEnum`) 1)))))))
    (else
      (return (`|GetEnumeratorNameAsString` (enumliteral `/Game/RTS/Enums/FemaleNameEnum` (cast `/Game/RTS/Enums/FemaleNameEnum` (`KismetMathLibrary.Conv_IntToByte` (`KismetMathLibrary.RandomIntegerInRange` 0 (- (enumcount `/Game/RTS/Enums/FemaleNameEnum`) 1))))))))))

(fn `RandomNPCFeatures`
  (locals (MaterialInstance :type "MaterialInstanceDynamic Object Reference") (FemaleColor :type "LinearColor Structure" :default (struct :`R` 0.588542 :`G` 0.146294 :`B` 0.295753)) (MaleColor :type "LinearColor Structure" :default (struct :`R` 0.24166 :`G` 0.422094 :`B` 0.654514)))
  (bind _materialinstance (`local.MaterialInstance`))
  (bind _returnvalue (`PrimitiveComponent.CreateDynamicMaterialInstance` (`self.Mesh`) 0 "/Game/Mannequin/Character/Materials/M_UE4Man_Body_Inst.M_UE4Man_Body_Inst" "None"))
  (set `local.MaterialInstance` _returnvalue)
  (switch `int` (`KismetMathLibrary.RandomIntegerInRange` 0 1)
    (:`0`
      (`MaterialInstanceDynamic.SetVectorParameterValue` _materialinstance "BodyColor" (`local.MaleColor`))
      (bind _name (`self.GetRandomName` 0))
      (set `self.MyProfile` (make `/Game/RTS/Structs/NPCProfile_Struct` _name)))
    (:`1`
      (`MaterialInstanceDynamic.SetVectorParameterValue` _materialinstance "BodyColor" (`local.FemaleColor`))
      (bind _name_2 (`self.GetRandomName` 0))
      (set `self.MyProfile` (make `/Game/RTS/Structs/NPCProfile_Struct` _name_2 0)))))

(fn `SetIsBusy`
  (params (IsBusy :type Boolean))
  (`BlackboardComponent.SetValueAsBool` (`AIBlueprintHelperLibrary.GetBlackboard` null) (`self.IsBusy`) IsBusy)
  (return))

(fn `UserConstructionScript`
  (`self.RandomNPCFeatures`))