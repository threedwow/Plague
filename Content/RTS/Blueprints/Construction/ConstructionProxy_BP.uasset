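; Construction proxy actor for the RTS that stands in for a building under construction and times its completion.
; The construction script shows the display mesh with a ghost material and sets up its entrance and collision box.
; Each tick accumulates work time from delta seconds and the game state's time unit.
; When that reaches the construction time, it signals completion and destroys itself after a short delay.
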(event `self.ReceiveTick`
  (params (DeltaSeconds :type "Float (single-precision)"))
  (set `self.Delta` DeltaSeconds)
  (set `self.TimeUnit` (`/Game/RTS/GameBP/MyGameState.TimeUnit` (`self.GameStateRef`)))
  (if (not (`self.IsConstructionCompleted`))
    (`self.DoWork`)
    (if (>= (`self.WorkTimeSpent`) (`self.ConstructionTime`))
      (set `self.IsConstructionCompleted` true)
      (`self.ConstructionCompleted` self)
      (`KismetSystemLibrary.Delay` 0.2)
      (`self.K2_DestroyActor`))))

(event `self.ReceiveBeginPlay`
  (bind _output_get (set `self.GameStateRef` (cast `/Game/RTS/GameBP/MyGameState` (`GameplayStatics.GetGameState`) :!pure true)))
  (add `/Game/RTS/GameBP/MyGameState.UpdateGameSpeed` _output_get (`|CreateDelegate` :!event `AdjustTime`)))

(event `AdjustTime`
  (params (TimeUnit :type "Float (double-precision)"))
  (set `self.TimeUnit` TimeUnit))

(fn `DoWork`
  (bind _output_get (set `self.ClockWork` (`/Game/RTS/Library/FunctionLibrary.SetClockWork` (`self.Delta`) (`self.TimeUnit`) (`self.ClockWork`))))
  (set `self.WorkTimeSpent` (* _output_get 60.0))
  (return))

(fn `SetConstructionTime`
  (params (WorkHours :type "Float (double-precision)"))
  (set `self.ConstructionTime` (* WorkHours 60.0))
  (return))

(fn `UserConstructionScript`
  (bind _staticmesh (`self.StaticMesh`))
  (`StaticMeshComponent.SetStaticMesh` _staticmesh (`self.DisplayMesh`))
  (`PrimitiveComponent.SetMaterial` _staticmesh 0 "/Game/RTS/Materials/Ghost_Buld_Success.Ghost_Buld_Success")
  (`/Game/RTS/Library/FunctionLibrary.SetBuildingEntrance` (`self.Entrance`) (`self.StaticMesh`))
  (`/Game/RTS/Library/FunctionLibrary.SetBuildingCollisionBox` (`self.Collision`) (`self.StaticMesh`)))