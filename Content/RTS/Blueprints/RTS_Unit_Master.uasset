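; RTS unit master Blueprint that gives each unit a random identity: sex, enum-based name, age, portrait and matching body colour via dynamic material.
; Spawned units roll features in the construction script and take the current game date as birthday; others roll at BeginPlay with a random birth date.
; BirthdayCheck increments age on that date.
; A controller event opens the unit's info widget and switches input to UI-only.
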(event `self.ReceiveBeginPlay`
  (`|ExecutionSequence`
    (:`then_0`
      (`self.ReferenceCast`)
      (add `/Game/RTS/Blueprints/CameraPawnController.DisplayUnitHud` (`self.ControllerRef`) (`|CreateDelegate` :!event `DisplayUnitHUD`)))
    (:`then_2`
      (if (not (`self.IsSpawnedIn`))
        (`self.SetUnitFeatures`)))
    (:`then_3`
      (`self.SetBirthday`))))

(event `BirthdayCheck`
  (bind _game_state_ref (`self.Game State Ref`))
  (if (and (== (`/Game/RTS/GameBP/MyGameState.Month` _game_state_ref) (`self.BirthMonth`)) (== (`/Game/RTS/GameBP/MyGameState.Day` _game_state_ref) (`self.BirthDay`)))
    (bind _result (`/Engine/EditorBlueprintResources/StandardMacros.IncrementInt` (`self.UnitAge`))
      (:`  `
        (set `self.UnitAge` _result)))))

(event `DisplayUnitHUD`
  (params (Actor :type "Actor Object Reference") (Bypass :type Boolean))
  (bind _controllerref (`self.ControllerRef`))
  (if (and (== Actor self) (or Bypass (not (`self.IsHidden`))))
    (`UserWidget.AddToViewport` (`self.Hud_Unit_Ref`) 1)
    (`WidgetBlueprintLibrary.SetInputMode_UIOnlyEx` _controllerref null)
    (`Widget.SetIsEnabled` (`/Game/RTS/Blueprints/CameraPawnController.MainHudRef` _controllerref) true)))

(fn `GetRandomName`
  (params (Sex :type Integer))
  (returns (UnitNmae :type String))
  (if (== Sex 0)
    (bind _output_get (set `self.MaleName` (`self.SetMaleName`)))
    (bind _output_get_2 (set `self.SirName` (`self.SetSirName`)))
    (return (`KismetStringLibrary.Concat_StrStr` (`|GetEnumeratorNameAsString` _output_get) " " (`|GetEnumeratorNameAsString` _output_get_2)))
    (else
      (bind _output_get_3 (set `self.FemaleName` (`self.SetFemaleName`)))
      (bind _output_get_4 (set `self.SirName` (`self.SetSirName`)))
      (return (`KismetStringLibrary.Concat_StrStr` (`|GetEnumeratorNameAsString` _output_get_3) " " (`|GetEnumeratorNameAsString` _output_get_4))))))

(fn `SetBirthday`
  (bind _game_state_ref (`self.Game State Ref`))
  (if (`self.IsSpawnedIn`)
    (set `self.BirthYear` (- (`/Game/RTS/GameBP/MyGameState.Year` _game_state_ref) (`self.UnitAge`)))
    (set `self.BirthDay` (`/Game/RTS/GameBP/MyGameState.Day` _game_state_ref))
    (set `self.BirthMonth` (`/Game/RTS/GameBP/MyGameState.Month` _game_state_ref))
    (else
      (set `self.BirthYear` (- (`/Game/RTS/GameBP/MyGameState.Year` _game_state_ref) (`self.UnitAge`)))
      (set `self.BirthMonth` (`KismetMathLibrary.RandomIntegerInRange` 1 12))
      (set `self.BirthDay` (`KismetMathLibrary.Clamp` (`KismetMathLibrary.RandomIntegerInRange` 1 31) 0 (`KismetMathLibrary.DaysInMonth` (`self.BirthYear`) (`self.BirthMonth`)))))))

(fn `SetUnitFeatures`
  (locals (MsehMaterialInstanceLocal :type "MaterialInstanceDynamic Object Reference") (NewLocalVar_0 :type Integer :default 0))
  (bind _unitimage (`self.UnitImage`))
  (bind _returnvalue (`PrimitiveComponent.CreateDynamicMaterialInstance` (`self.Mesh`) 0 null "None"))
  (set `local.MsehMaterialInstanceLocal` _returnvalue)
  (set `self.UnitSex` (`KismetMathLibrary.RandomIntegerInRange` 0 1))
  (if (== (`self.UnitSex`) 0)
    (`MaterialInstanceDynamic.SetVectorParameterValue` (`local.MsehMaterialInstanceLocal`) "BodyColor" (struct :`B` 1.0 :`A` 1.0))
    (bind _unitnmae (`self.GetRandomName` (`self.UnitSex`)))
    (set `self.UnitName` _unitnmae)
    (set `self.UnitAge` (`KismetMathLibrary.RandomIntegerInRange` 18 70))
    (set `self.UnitImage` (`self.MaleImage`))
    (set `self.UnitProfile` (make `/Game/RTS/Blueprints/Structures/RTS_UnitProfileStruct` (`self.UnitName`) (`self.UnitSex`) (`self.UnitAge`) _unitimage))
    (else
      (`MaterialInstanceDynamic.SetVectorParameterValue` (`local.MsehMaterialInstanceLocal`) "BodyColor" (struct :`R` 0.984243 :`B` 1.0 :`A` 1.0))
      (bind _unitnmae_2 (`self.GetRandomName` (`self.UnitSex`)))
      (set `self.UnitName` _unitnmae_2)
      (set `self.UnitAge` (`KismetMathLibrary.RandomIntegerInRange` 18 70))
      (set `self.UnitImage` (`self.FemaleImage`))
      (set `self.UnitProfile` (make `/Game/RTS/Blueprints/Structures/RTS_UnitProfileStruct` (`self.UnitName`) (`self.UnitSex`) (`self.UnitAge`) _unitimage)))))

(fn `UserConstructionScript`
  (if (`self.IsSpawnedIn`)
    (`self.SetUnitFeatures`)))