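; RTS player controller that drives the camera pawn, creates the main HUD and positions a building placement preview.
; Input pans with keys or screen edges, rotates through gated mouse look, and zooms the spring arm, whose length scales key movement speed.
; In building mode, Tick moves the spawned preview to the cursor and input rotates it; V spawns an NPC there.
; Placement cancel and click-selection logic is present but unconnected.
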(event `InputAction|Deselect`
  (params (Key :type "Key Structure"))
  ;[1 1 1] Cancel Building Placement
)

(event `Key|LeftMouseButton`
  (params (Key :type "Key Structure")))

(event `self.ReceiveBeginPlay`
  ;[1 1 1] Mouse / Viewport
  (`|ExecutionSequence`
    (:`then_0`
      (`self.ReferenceCasts`))
    (:`then_1`
      (bind _returnvalue (`|SpawnActorFromClass` "/Game/RTS/Blueprints/Buildings/RTS_PreviewBuilding.RTS_PreviewBuilding_C" (`self.EmptyTransform`) "AlwaysSpawn" "OverrideRootScale" null self null))
      (set `self.ContructionPreview` _returnvalue))
    (:`then_2`
      (`WidgetBlueprintLibrary.SetInputMode_GameAndUIEx` self null "LockAlways" false)
      (`self.CreateHuds`)
      (`UserWidget.AddToViewport` (`self.MainHudRef`) 0))))

(event `InputAction|RotateBuildingRight`
  (params (Key :type "Key Structure"))
  (bind _contructionpreview (`self.ContructionPreview`))
  ;[1 1 1] BuildingPlacement
  (:`Pressed`
    (if (and (`KismetSystemLibrary.IsValid` _contructionpreview) (`self.IsBuildingModeActive`))
      (`self.K2_SetActorRotation` _contructionpreview (`KismetMathLibrary.MakeRotator` (.roll (`self.K2_GetActorRotation` _contructionpreview)) (.pitch (`self.K2_GetActorRotation` _contructionpreview)) (- (.yaw (`self.K2_GetActorRotation` _contructionpreview)) (`self.BuildingRotationRate`))) false))))

(event `InputAction|RotateBuildingLeft`
  (params (Key :type "Key Structure"))
  (bind _contructionpreview (`self.ContructionPreview`))
  ;[1 1 1] BuildingPlacement
  (:`Pressed`
    (if (and (`KismetSystemLibrary.IsValid` _contructionpreview) (`self.IsBuildingModeActive`))
      (`self.K2_SetActorRotation` (`KismetMathLibrary.MakeRotator` (.roll (`self.K2_GetActorRotation` _contructionpreview)) (.pitch (`self.K2_GetActorRotation` _contructionpreview)) (+ (.yaw (`self.K2_GetActorRotation` _contructionpreview)) (`self.BuildingRotationRate`)))))))

(event `self.ReceiveTick`
  (params (DeltaSeconds :type "Float (single-precision)"))
  ;[1 1 1] Cursor Location
  (set `self.DeltaTime` DeltaSeconds)
  (if (`self.BuildModeActive`)
    _
    (elif (and (`self.IsBuildingModeActive`) (!= (`self.ContructionPreview`) null))
      (`/Game/RTS/Blueprints/Buildings/RTS_PreviewBuilding.GetCursorPosition` (`self.ContructionPreview`) (`/Game/RTS/Library/FunctionLibrary.SetCursorWorldPosition` self 10000.0)))))

(event `Key|V`
  (params (Key :type "Key Structure"))
  (bind (_location_x _location_y) (`KismetMathLibrary.BreakVector` (`/Game/RTS/Library/FunctionLibrary.SetCursorWorldPosition` self 10000.0)))
  (:`Pressed`
    (`|SpawnActorFromClass` "/Game/RTS/AI/NPC_BP.NPC_BP_C" (`KismetMathLibrary.MakeTransform` (`KismetMathLibrary.MakeVector` _location_x _location_y 90.0)) "Undefined" "OverrideRootScale" null null)))

(event `InputAxis|MoveForward`
  (params (AxisValue :type "Float (single-precision)"))
  (bind _camerapawnref (`self.CameraPawnRef`))
  ;[1 1 1] Camera Movement
  ;;[1 1 1] Movement X
  (if (not (`self.DisableCamNav`))
    (`self.K2_SetActorTransform` _camerapawnref (`KismetMathLibrary.MakeTransform` (`KismetMathLibrary.MakeVector` (.x (.location (`self.MovementX` (`self.MovementSpeedCalculation`) (`self.FastMoveMultiplier`) AxisValue _camerapawnref))) (.y (.location (`self.MovementX` (`self.MovementSpeedCalculation`) (`self.FastMoveMultiplier`) AxisValue _camerapawnref))) 100.0) (.rotation (`self.MovementX` (`self.MovementSpeedCalculation`) (`self.FastMoveMultiplier`) AxisValue _camerapawnref)) (.scale (`self.MovementX` (`self.MovementSpeedCalculation`) (`self.FastMoveMultiplier`) AxisValue _camerapawnref))) false false)))

(event `InputAxis|MoveRight`
  (params (AxisValue :type "Float (single-precision)"))
  (bind _camerapawnref (`self.CameraPawnRef`))
  ;[1 1 1] Camera Movement
  ;;[1 1 1] Movement Y
  (if (not (`self.DisableCamNav`))
    (`self.K2_SetActorTransform` _camerapawnref (`KismetMathLibrary.MakeTransform` (`KismetMathLibrary.MakeVector` (.x (.location (`self.MovementY` (`self.MovementSpeedCalculation`) (`self.FastMoveMultiplier`) AxisValue _camerapawnref))) (.y (.location (`self.MovementY` (`self.MovementSpeedCalculation`) (`self.FastMoveMultiplier`) AxisValue _camerapawnref))) 100.0) (.rotation (`self.MovementY` (`self.MovementSpeedCalculation`) (`self.FastMoveMultiplier`) AxisValue _camerapawnref)) (.scale (`self.MovementY` (`self.MovementSpeedCalculation`) (`self.FastMoveMultiplier`) AxisValue _camerapawnref))) false false)))

(event `InputAction|PanReset`
  (params (Key :type "Key Structure"))
  (bind _camerapawnref (`self.CameraPawnRef`))
  ;[1 1 1] Camera Movement
  ;;[1 1 1] Pan Reset
  (:`Pressed`
    (`self.K2_SetActorRotation` _camerapawnref (`KismetMathLibrary.MakeRotator` (.roll (`self.K2_GetActorRotation` _camerapawnref)) 0.0 (.yaw (`self.K2_GetActorRotation` _camerapawnref))) false)))

(event `InputAxisKey|MouseX`
  (params (AxisValue :type "Float (single-precision)"))
  (bind _camerapawnref (`self.CameraPawnRef`))
  ;[1 1 1] Camera Movement
  ;;[1 1 1] Pan X
  (`/Engine/EditorBlueprintResources/StandardMacros.Gate` true :!label _label
    (:`Exit`
      (`self.K2_SetActorRotation` _camerapawnref (`KismetMathLibrary.MakeRotator` (.roll (`self.K2_GetActorRotation` _camerapawnref)) (.pitch (`self.K2_GetActorRotation` _camerapawnref)) (+ (.yaw (`self.K2_GetActorRotation` _camerapawnref)) (* (`self.PanSensitivity`) AxisValue))) false))))

(event `InputAction|Pan`
  (params (Key :type "Key Structure"))
  ;[1 1 1] Camera Movement
  ;;[1 1 1] Pan X
  (:`Pressed`
    (set `self.DisableCamNav` true)
    (goto _label :!via `Open`))
  (:`Released`
    (set `self.DisableCamNav` false)
    (goto _label :!via `Close`)))

(event `Key|LeftShift`
  (params (Key :type "Key Structure"))
  ;[1 1 1] Camera Movement
  ;;[1 1 1] Faster Panning
  (:`Pressed`
    (set `self.FastMoveMultiplier` 2.0))
  (:`Released`
    (set `self.FastMoveMultiplier` 1.0)))

(event `InputAxisKey|MouseY`
  (params (AxisValue :type "Float (single-precision)"))
  (bind _camerapawnref (`self.CameraPawnRef`))
  ;[1 1 1] Camera Movement
  ;;[1 1 1] Pan Y
  (`/Engine/EditorBlueprintResources/StandardMacros.Gate` true :!label _label_2
    (:`Exit`
      (`self.K2_SetActorRotation` _camerapawnref (`KismetMathLibrary.MakeRotator` (.roll (`self.K2_GetActorRotation` _camerapawnref)) (`KismetMathLibrary.FClamp` (+ (.pitch (`self.K2_GetActorRotation` _camerapawnref)) (* (`self.PanSensitivity`) AxisValue)) -15.0 45.0) (.yaw (`self.K2_GetActorRotation` _camerapawnref))) false))))

(event `InputAction|Pan`
  (params (Key :type "Key Structure"))
  ;[1 1 1] Camera Movement
  ;;[1 1 1] Pan Y
  (:`Pressed`
    (set `self.DisableCamNav` true)
    (goto _label_2 :!via `Open`))
  (:`Released`
    (set `self.DisableCamNav` false)
    (goto _label_2 :!via `Close`)))

(event `InputAction|ZoomIn`
  (params (Key :type "Key Structure"))
  (bind _springarm (`/Game/RTS/Blueprints/CameraPawn.SpringArm` (`self.CameraPawnRef`)))
  ;[1 1 1] Camera Movement
  ;;[1 1 1] Zoom In / Out
  (:`Pressed`
    (set `SpringArmComponent.TargetArmLength` (`KismetMathLibrary.FClamp` (- (`SpringArmComponent.TargetArmLength` _springarm) (`self.ZoomSensitivity`)) 1000.0 (`self.MaxArmDistance`)) _springarm)))

(event `InputAction|ZoomReset`
  (params (Key :type "Key Structure"))
  ;[1 1 1] Camera Movement
  ;;[1 1 1] Zoom Reset
  (:`Pressed`
    (set `SpringArmComponent.TargetArmLength` 1500.0 (`/Game/RTS/Blueprints/CameraPawn.SpringArm` (`self.CameraPawnRef`)))))

(event `InputAction|ZoomOut`
  (params (Key :type "Key Structure"))
  (bind _springarm (`/Game/RTS/Blueprints/CameraPawn.SpringArm` (`self.CameraPawnRef`)))
  ;[1 1 1] Camera Movement
  ;;[1 1 1] Zoom In / Out
  (:`Pressed`
    (set `SpringArmComponent.TargetArmLength` (`KismetMathLibrary.FClamp` (+ (`self.ZoomSensitivity`) (`SpringArmComponent.TargetArmLength` _springarm)) 500.0 (`self.MaxArmDistance`)) _springarm)))

(event `InputAxisKey|MouseX`
  (params (AxisValue :type "Float (single-precision)"))
  ;[1 1 1] Camera Movement
  ;;[1 1 1] Edge Movement
  (if (not (`self.DisableCamNav`))
    (bind (_deltaxspeed _deltayspeed) (`self.ScreenEdgeMovement` :!label _label_3))
    (`self.K2_AddActorLocalOffset` (`self.CameraPawnRef`) (`KismetMathLibrary.MakeVector` _deltaxspeed _deltayspeed) true false)))

(event `InputAxisKey|MouseY`
  (params (AxisValue :type "Float (single-precision)"))
  ;[1 1 1] Camera Movement
  ;;[1 1 1] Edge Movement
  (if (not (`self.DisableCamNav`))
    (goto _label_3 :!via `MouseY`)))

(fn `MovementSpeedCalculation`
  (returns (MoveSensitivity :type "Float (double-precision)"))
  (return (`KismetMathLibrary.FClamp` (/ (`SpringArmComponent.TargetArmLength` (`/Game/RTS/Blueprints/CameraPawn.SpringArm` (`self.CameraPawnRef`))) 100.0) 5.0 20.0)))

(fn `SetBuildingModeActive`
  (params (IsActive :type Boolean))
  (set `self.IsBuildingModeActive` IsActive)
  (return))

(fn `SetCalendar`
  (params (Date :type "Array of Integer (by ref)"))
  (returns (Success :type Boolean))
  (return false))

(fn `SetClock`
  (params (Time :type "Array of Integer (by ref)"))
  (returns (Success :type Boolean))
  (return false))

(fn `SetSightDistance`
  (returns (SightDistance :type "Float (double-precision)"))
  (return (+ (`self.SightDistance`) (`SpringArmComponent.TargetArmLength` (`/Game/RTS/Blueprints/CameraPawn.SpringArm` (`self.CameraPawnRef`))))))

(fn `UserConstructionScript`)