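; Base RTS building Blueprint that tracks the game speed and holds basic construction state.
; On BeginPlay it caches the MyGameState reference, binds to its game speed updates and reads the current value.
; The construction script applies the display mesh, while OnSpawn flags the building as under construction.
; Tick stores delta time and sets TimeWorked to the current game time; construction progress logic is not implemented here.
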(event `self.ReceiveBeginPlay`
  (`|ExecutionSequence`
    (:`then_0`
      (`self.RefCasts`))
    (:`then_1`
      (add `/Game/RTS/GameBP/MyGameState.UpdateGameSpeed` (`self.GameStateRef`) (`|CreateDelegate` :!event `GetGameSpeed`))
      (bind _gamespeed (`/Game/RTS/GameBP/MyGameState.GameSpeed` (`self.GameStateRef`)))
      (set `self.GameSpeed` _gamespeed))))

(event `OnSpawn`
  (set `self.IsUnderConstruction` true))

(event `GetGameSpeed`
  (params (GameSpeed :type "Float (double-precision)"))
  (set `self.GameSpeed` GameSpeed))

(event `self.ReceiveTick`
  (params (DeltaSeconds :type "Float (single-precision)"))
  (set `self.DeltaTime` DeltaSeconds)
  (if true
    (set `self.TimeWorked` (`KismetSystemLibrary.GetGameTimeInSeconds`))))

(fn `UserConstructionScript`
  (`StaticMeshComponent.SetStaticMesh` (`self.BuildingMesh`) (`self.DisplayMesh`))
  (if (`self.IsBuilt`)
    _))