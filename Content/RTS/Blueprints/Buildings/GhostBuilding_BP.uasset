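; Ghost building for RTS build mode that previews a structure at the cursor and flags invalid placement.
; ConstructBuilding briefly spawns the building class to read its mesh, proxy and work hours, then restarts the ghost.
; A gated Tick grid-snaps the ghost, switching to an error material on overlap or steep slope.
; Slope uses corner and center line traces, plus a box trace for height; GetConstructionStruct packages the placement data.
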(event `OnSpawn`
  (params (DisplayMesh :type "StaticMesh Object Reference") (BuildingClass :type "/Game/RTS/Blueprints/Buildings/BuildingMaster_BP Class Reference") (ConstructionProxy :type "/Game/RTS/Blueprints/Construction/ConstructionProxy_BP Class Reference") (WorkHours :type "Float (double-precision)"))
  (bind _ghostbuilding_mesh (`self.GhostBuilding_Mesh`))
  (bind _arrow (`self.Arrow`))
  ;[1 1 1] On Spawn Ghost
  (if (not (`self.IsActive`))
    (set `self.BuildingClass` BuildingClass)
    (set `self.ConstructionProxy` ConstructionProxy)
    (set `self.DisplayMesh` DisplayMesh)
    (set `self.WorkHoursRequired` WorkHours)
    (set `self.IsActive` true)
    (set `/Game/RTS/Blueprints/CameraPawnController.BuildModeActive` true (`self.ControllerRef`))
    (`StaticMeshComponent.SetStaticMesh` _ghostbuilding_mesh (`self.DisplayMesh`))
    (`self.OpenTickGate`)
    (`self.SetMaterial` (not (`self.IsOverlapping`)))
    (bind _output_get (set `self.Extent` (`.BoxExtent` (`KismetSystemLibrary.GetComponentBounds` _ghostbuilding_mesh))))
    (`SceneComponent.K2_SetRelativeLocation` _arrow (`KismetMathLibrary.MakeVector` (.x _output_get)) false false)
    (`SceneComponent.SetHiddenInGame` _arrow false false)
    (`/Game/RTS/Library/FunctionLibrary.SetBuildingCollisionBox` (`self.Collision`) (`self.GhostBuilding_Mesh`))))

(event `KillGhost`
  ;[1 1 1] Kill Ghost
  (set `self.BuildingClass` null)
  (set `self.ConstructionProxy` null)
  (`self.ClosedTickGate`)
  (set `self.DisplayMesh` null)
  (set `self.IsActive` false)
  (set `/Game/RTS/Blueprints/CameraPawnController.BuildModeActive` false (`self.ControllerRef`))
  (`StaticMeshComponent.SetStaticMesh` (`self.GhostBuilding_Mesh`) (`self.DisplayMesh`))
  (`self.K2_SetActorRotation` (struct))
  (`SceneComponent.SetHiddenInGame` (`self.Arrow`) true false))

(event `/Game/RTS/Interfaces/I_HUD.ConstructBuilding`
  (params (MainBuilding :type "/Game/RTS/Blueprints/Buildings/BuildingMaster_BP Class Reference"))
  ;[1 1 1] Construct Building
  (bind _returnvalue (`|SpawnActorFromClass` MainBuilding (`KismetMathLibrary.MakeTransform` (0.0 0.0 0.0)) "Undefined" "OverrideRootScale" null (`self.ControllerRef`) null))
  (`|ExecutionSequence`
    (:`then_0`
      (bind _asbuilding_master_bp (castclass `/Game/RTS/Blueprints/Buildings/BuildingMaster_BP` MainBuilding))
      (`self.KillGhost` self)
      (`self.OnSpawn` (`/Game/RTS/Blueprints/Buildings/BuildingMaster_BP.DisplayMesh` _returnvalue) _asbuilding_master_bp (`/Game/RTS/Blueprints/Buildings/BuildingMaster_BP.ConstructionProxy` _returnvalue) (`/Game/RTS/Blueprints/Buildings/BuildingMaster_BP.ConstructionTime` _returnvalue)))
    (:`then_1`
      (`self.K2_DestroyActor` _returnvalue))))

(event `self.ReceiveTick`
  (params (DeltaSeconds :type "Float (single-precision)"))
  ;[1 1 1] Placemen tOverlap Materials
  (`/Engine/EditorBlueprintResources/StandardMacros.Gate` true :!label _label
    (:`Exit`
      (`self.K2_SetActorLocation` self (`self.SetGridSnapVector`) false false)
      (if (`self.CheckOverlap`)
        (`self.SetMaterial` true)
        (else
          (bind _badlocation (`self.CalculateSlope`))
          (`self.SetMaterial` _badlocation))))))

(event `OpenTickGate`
  ;[1 1 1] Placemen tOverlap Materials
  (goto _label :!via `Open`))

(event `ClosedTickGate`
  ;[1 1 1] Placemen tOverlap Materials
  (goto _label :!via `Close`))

(event `SetMaterial`
  (params (IsError :type Boolean))
  (bind _ghostbuilding_mesh (`self.GhostBuilding_Mesh`))
  ;[1 1 1] Placemen tOverlap Materials
  (if (not (== IsError (`self.IsOverlapping`)))
    (bind _output_get (set `self.IsOverlapping` IsError))
    (if _output_get
      (`PrimitiveComponent.SetMaterial` _ghostbuilding_mesh 0 "/Game/RTS/Materials/Ghost_Build_Error.Ghost_Build_Error")
      (else
        (`PrimitiveComponent.SetMaterial` _ghostbuilding_mesh 0 "/Game/StarterContent/Materials/M_Basic_Floor.M_Basic_Floor")))))

(fn `CalculateSlope`
  (returns (BadLocation :type Boolean))
  (locals (Differences :type "Array of Float (double-precision)") (MaxDifferences :type "Float (double-precision)" :default 20.0))
  (bind (_actorlocation _forwardvector _rightvector) (`self.GetVectors`))
  (bind (_actorlocation_2 _forwardvector_2 _rightvector_2) (`self.GetVectors`))
  (bind _actorlocation_3 (`self.GetVectors`))
  (bind _actorlocation_4 (`self.GetVectors`))
  (bind (_actorlocation_5 _forwardvector_3 _rightvector_3) (`self.GetVectors`))
  (bind (_actorlocation_6 _forwardvector_4 _rightvector_4) (`self.GetVectors`))
  (bind _extent (`self.Extent`))
  (bind _differences (`local.Differences`))
  (bind (_extent_x _extent_y) (`KismetMathLibrary.BreakVector` (`self.Extent`)))
  (bind _maxdifferences (`local.MaxDifferences`))
  (bind (_indexofminvalue _minvalue) (`KismetMathLibrary.MinOfFloatArray` _differences))
  (bind (_indexofmaxvalue _maxvalue) (`KismetMathLibrary.MaxOfFloatArray` _differences))
  (`|ExecutionSequence`
    (:`then_0`
      (`|ExecutionSequence`
        (:`then_0`
          (bind _difference (`self.SlopeTrace` (+ _actorlocation_5 (* (+ _forwardvector_3 _rightvector_3) _extent))))
          (`KismetArrayLibrary.Array_Add` (`local.Differences`) _difference))
        (:`then_1`
          (bind _difference_2 (`self.SlopeTrace` (+ _actorlocation_6 (* (+ (* _forwardvector_4 -1.0) _rightvector_4) _extent))))
          (`KismetArrayLibrary.Array_Add` (`local.Differences`) _difference_2))
        (:`then_2`
          (bind _difference_3 (`self.SlopeTrace` (+ _actorlocation (* (+ _forwardvector (* _rightvector -1.0)) _extent))))
          (`KismetArrayLibrary.Array_Add` (`local.Differences`) _difference_3))
        (:`then_3`
          (bind _difference_4 (`self.SlopeTrace` (+ _actorlocation_2 (* (+ (* _forwardvector_2 -1.0) (* _rightvector_2 -1.0)) _extent))))
          (`KismetArrayLibrary.Array_Add` (`local.Differences`) _difference_4))
        (:`then_4`
          (bind _difference_5 (`self.SlopeTrace` (`self.GetVectors`)))
          (`KismetArrayLibrary.Array_Add` (`local.Differences`) _difference_5))))
    (:`then_1`
      (if (and (> _indexofminvalue -1) (> _indexofmaxvalue -1))
        (bind (_outhit _returnvalue) (`KismetSystemLibrary.BoxTraceSingle` (+ _actorlocation_3 (0.0 0.0 1000.0)) (- _actorlocation_3 (0.0 0.0 100.0)) (`KismetMathLibrary.MakeVector` _extent_x _extent_y 1.0) (struct) "TraceTypeQuery3"))
        (if _returnvalue
          (`self.K2_SetActorLocation` (`KismetMathLibrary.MakeVector` (.x _actorlocation_4) (.y _actorlocation_4) (.z (`.ImpactPoint` (`GameplayStatics.BreakHitResult` _outhit))))))))
    (:`then_2`
      (return (or (> (`KismetMathLibrary.Abs` _minvalue) _maxdifferences) (> (`KismetMathLibrary.Abs` _maxvalue) _maxdifferences))))))

(fn `CheckOverlap`
  (returns (Overlapping :type Boolean))
  (return (> (`KismetArrayLibrary.Array_Length` (`self.GetOverlappingActors` "/Script/Engine.Actor")) 0)))

(fn `GetConstructionStruct`
  (returns (ConstructionStruct :type "/Game/RTS/Structs/Construction_Struct Structure"))
  (return (make `/Game/RTS/Structs/Construction_Struct` (`self.BuildingClass`) (`self.ConstructionProxy`) (`KismetMathLibrary.MakeTransform` (`self.K2_GetActorLocation`) (`self.K2_GetActorRotation`)) (`self.DisplayMesh`) (`self.WorkHoursRequired`))))

(fn `GetIsOverlapping`
  (returns (IsOverlapping :type Boolean))
  (return (`self.IsOverlapping`)))

(fn `GetVectors`
  (returns (ActorLocation :type "Vector Structure") (ForwardVector :type "Vector Structure") (RightVector :type "Vector Structure"))
  (bind _returnvalue (`self.K2_GetActorRotation`))
  (return (`self.K2_GetActorLocation`) (`KismetMathLibrary.GetForwardVector` _returnvalue) (`KismetMathLibrary.GetRightVector` _returnvalue)))

(fn `SetCalendar`
  (params (Date :type "Array of Integer (by ref)"))
  (returns (Success :type Boolean))
  (return false))

(fn `SetClock`
  (params (Time :type "Array of Integer (by ref)"))
  (returns (Success :type Boolean))
  (return false))

(fn `SetCursorPostion`
  (params (CursorLocation :type "Vector Structure"))
  (set `self.CursorWorldPosition` CursorLocation)
  (return))

(fn `SetGridSnapVector`
  (returns (GridSnap :type "Vector Structure"))
  (bind (_cursorworldposition_x _cursorworldposition_y _cursorworldposition_z) (`KismetMathLibrary.BreakVector` (`self.CursorWorldPosition`)))
  (bind _gridsize (`self.GridSize`))
  (return (`KismetMathLibrary.MakeVector` (`/Game/RTS/Library/FunctionLibrary.GridSnap` _cursorworldposition_x _gridsize) (`/Game/RTS/Library/FunctionLibrary.GridSnap` _cursorworldposition_y _gridsize) (`/Game/RTS/Library/FunctionLibrary.GridSnap` _cursorworldposition_z _gridsize))))

(fn `SlopeTrace`
  (params (TraceLocation :type "Vector Structure"))
  (returns (Difference :type "Float (double-precision)"))
  (bind (_returnvalue_x _returnvalue_y _returnvalue_z) (`KismetMathLibrary.BreakVector` (`self.K2_GetActorLocation`)))
  (bind (_returnvalue_min _returnvalue_max) (break `Box` (`StaticMesh.GetBoundingBox` (`StaticMeshComponent.StaticMesh` (`self.GhostBuilding_Mesh`)))))
  (bind _returnvalue (+ TraceLocation (+ (+ _returnvalue_min _returnvalue_max) 0.0)))
  (bind _outhit (`KismetSystemLibrary.LineTraceSingle` (+ _returnvalue (0.0 0.0 1000.0)) (- _returnvalue (0.0 0.0 1000.0)) "TraceTypeQuery3"))
  (return (- _returnvalue_z (.z (`.ImpactPoint` (`GameplayStatics.BreakHitResult` _outhit))))))

(fn `UserConstructionScript`)