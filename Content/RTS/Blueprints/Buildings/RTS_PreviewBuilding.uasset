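; Ghost preview actor for RTS building placement, showing the selected building's mesh while notifying the player controller about building mode.
; ConstructionBuilding briefly spawns the building class to read its display mesh for SpawnPreview.
; A gated Tick snaps the preview to a grid under the supplied cursor position and switches to an error material on actor overlap.
; SetConStructionStructure packages class, transform, mesh and build time into a construction struct.
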(event `SpawnPreview`
  (params (BuildingClass :type "/Game/RTS/Blueprints/Buildings/RTS_BuildingMaster_BP Class Reference") (DisplayMesh :type "StaticMesh Object Reference"))
  (if (`self.IsPreviewing`)
    (`self.DestroyPreview`))
  (set `self.BuildingClass` BuildingClass)
  (set `self.DisplayMesh` DisplayMesh)
  (bind _output_get (set `self.IsPreviewing` true))
  (`/Game/RTS/Blueprints/CameraPawnController.SetBuildingModeActive` (`self.PlayerControllerRef`) _output_get)
  (`StaticMeshComponent.SetStaticMesh` (`self.PreviewBuildingMesh`) (`self.DisplayMesh`))
  (`self.OpenGate`))

(event `DestroyPreview`
  (`self.CloseGate`)
  (set `self.BuildingClass` null)
  (set `self.DisplayMesh` null)
  (bind _output_get (set `self.IsPreviewing` true))
  (`/Game/RTS/Blueprints/CameraPawnController.SetBuildingModeActive` (`self.PlayerControllerRef`) _output_get)
  (`StaticMeshComponent.SetStaticMesh` (`self.PreviewBuildingMesh`) (`self.DisplayMesh`))
  (`self.K2_SetActorRotation` (struct)))

(event `/Game/RTS/RTS_Construction_I.ConstructionBuilding`
  (params (BuildingMasterClass :type "/Game/RTS/Blueprints/Buildings/RTS_BuildingMaster_BP Class Reference"))
  (bind _returnvalue (`|SpawnActorFromClass` BuildingMasterClass (`self.EmptyTransform`) "AlwaysSpawn" "OverrideRootScale" null (`self.PlayerControllerRef`) null null))
  (`|ExecutionSequence`
    (:`then_0`
      (bind _asrts_building_master_bp (castclass `/Game/RTS/Blueprints/Buildings/RTS_BuildingMaster_BP` BuildingMasterClass))
      (`self.DestroyPreview`)
      (`self.SpawnPreview` _asrts_building_master_bp (`/Game/RTS/Blueprints/Buildings/RTS_BuildingMaster_BP.DisplayMesh` _returnvalue)))
    (:`then_1`
      (`self.K2_DestroyActor` _returnvalue))))

(event `self.ReceiveTick`
  (params (DeltaSeconds :type "Float (single-precision)"))
  (bind _previewbuildingmesh (`self.PreviewBuildingMesh`))
  (`/Engine/EditorBlueprintResources/StandardMacros.Gate` true :!label _label
    (:`Exit`
      (`self.K2_SetActorLocation` self (`self.GridSnaps`) false false)
      (if (`self.CheckOverlap`)
        (`PrimitiveComponent.SetMaterial` _previewbuildingmesh 0 "/Game/RTS/Materials/Ghost_Build_Error.Ghost_Build_Error")
        (else
          (`PrimitiveComponent.SetMaterial` _previewbuildingmesh 0 "/Game/RTS/Meshes/Leaves_Mat.Leaves_Mat"))))))

(event `OpenGate`
  (goto _label :!via `Open`))

(event `CloseGate`
  (goto _label :!via `Close`))

(fn `CheckOverlap`
  (returns (IsOverlapping :type Boolean))
  (return (>= (`KismetArrayLibrary.Array_LastIndex` (`self.GetOverlappingActors` null)) 0)))

(fn `GetCursorPosition`
  (params (CusorLocationIn :type "Vector Structure"))
  (set `self.CursorWorldPosition` CusorLocationIn)
  (return))

(fn `GridSnaps`
  (returns (SnapPosition :type "Vector Structure"))
  (bind (_cursorworldposition_x _cursorworldposition_y _cursorworldposition_z) (`KismetMathLibrary.BreakVector` (`self.CursorWorldPosition`)))
  (bind _snapvalue (`self.SnapValue`))
  (bind _snapvalue_2 (`self.SnapValue`))
  (return (`KismetMathLibrary.MakeVector` (`KismetMathLibrary.Conv_IntToDouble` (* (/ (`KismetMathLibrary.FFloor` (+ _cursorworldposition_x 50.0)) _snapvalue_2) _snapvalue_2)) (`KismetMathLibrary.Conv_IntToDouble` (* (/ (`KismetMathLibrary.FFloor` (+ _cursorworldposition_y 50.0)) _snapvalue) _snapvalue)) _cursorworldposition_z)))

(fn `SetConStructionStructure`
  (returns (ConstructionStruct :type "/Game/RTS/Structs/Construction_Struct Structure"))
  (set `self.ConstructionStruct` (make `/Game/RTS/Structs/Construction_Struct` false (`self.BuildingClass`) (`KismetMathLibrary.MakeTransform` (`self.K2_GetActorLocation`) (`self.K2_GetActorRotation`)) (`self.DisplayMesh`) (`self.ConstructionHours`)))
  (return (`self.ConstructionStruct`)))

(fn `UserConstructionScript`
  (`StaticMeshComponent.SetStaticMesh` (`self.PreviewBuildingMesh`) (`self.DisplayMesh`)))