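; Actor Blueprint that rotates a referenced sun actor to animate sun movement in the RTS, scaled by game speed.
; It reads game speed from MyGameState on BeginPlay and binds to its speed-control event to stay updated.
; Each Tick, SetGameTime converts delta time and speed into a time value that drives a local pitch rotation, then the sky sphere refreshes its sun direction.
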(event `self.ReceiveBeginPlay`
  (bind _game_state_ref (`self.Game State Ref`))
  (set `self.Game State Ref` (cast `/Game/RTS/GameBP/MyGameState` (`GameplayStatics.GetGameState`) :!pure true))
  (add `/Game/RTS/GameBP/MyGameState.GameSpeedControls` _game_state_ref (`|CreateDelegate` :!event `GetGameSpeed`))
  (bind _gamespeed (`/Game/RTS/GameBP/MyGameState.GetGameSpeed` _game_state_ref))
  (set `self.GameSpeed` _gamespeed))

(event `GetGameSpeed`
  (params (GameSpeed :type "Float (double-precision)"))
  (set `self.GameSpeed` GameSpeed))

(event `self.ReceiveTick`
  (params (DeltaSeconds :type "Float (single-precision)"))
  (`self.K2_AddActorLocalRotation` (`self.SunRef`) (`KismetMathLibrary.MakeRotator` 0.0 (* (/ (/ (`/Game/RTS/Library/FunctionLibrary.Set Game Time` DeltaSeconds (`self.GameSpeed`) (`self.Time`)) 1.5) 6.0) 90.0)) false false)
  (`/Engine/EngineSky/BP_Sky_Sphere.UpdateSunDirection` (`self.SkySphereRef`)))

(fn `UserConstructionScript`)